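; BP_DeathTalkSkull is a skull talk actor that damages the player when its talk finishes.
; FinishTalk casts the first player pawn to RedemptionPlayer and applies a small fixed amount of generic damage, with the player as its own damage causer.
; The graph holds no other active logic, and the construction script only calls its parent.
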(event `self.FinishTalk`
  (bind _asredemption_player (cast `RedemptionPlayer` (`GameplayStatics.GetPlayerPawn` 0)))
  (`GameplayStatics.ApplyDamage` _asredemption_player 2.0 (`GameplayStatics.GetPlayerController` 0) _asredemption_player "/Script/Engine.DamageType"))

(fn `UserConstructionScript`
  (`parent.UserConstructionScript`))