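; Game instance for Redemption that saves and loads persistent data through the single "RedemptionSave" slot.
; Saving runs SetupSaveInfo and copies SaveInfo into the existing SaveData, but a newly created save is written without that copy.
; Loading reads SaveInfo, creating a default save if needed, then runs TransferInfoSaveToInstance.
; It then applies music and SFX volumes as sound class overrides and pushes the game sound mix.
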(event `self.SaveGame`
  (`self.GameSave`))

(event `self.LoadGame`
  (`self.GameLoad`)
  (`KismetSystemLibrary.PrintString` "Loaded"))

(fn `GameLoad`
  (bind _returnvalue (`GameplayStatics.DoesSaveGameExist` "RedemptionSave"))
  (if _returnvalue
    (bind _returnvalue_2 (`GameplayStatics.LoadGameFromSlot` "RedemptionSave"))
    (bind _assave_data (cast `SaveData` _returnvalue_2)
      (:`then`
        (set `self.SaveInfo` (`SaveData.SaveDataStruct` _assave_data)))
      (:`CastFailed`
        (bind _returnvalue_3 (`GameplayStatics.CreateSaveGameObject` "/Script/Redemption.SaveData" :!label _label))
        (`GameplayStatics.SaveGameToSlot` _returnvalue_3 "RedemptionSave")
        (set `self.SaveInfo` (`SaveData.SaveDataStruct` _returnvalue_3))))
    (else
      (goto _label)))
  (`self.TransferInfoSaveToInstance`)
  (`GameplayStatics.SetSoundMixClassOverride` "/Game/Assets/Sounds/GameSoundClassMix.GameSoundClassMix" "/Game/Assets/Sounds/MusicSoundClass.MusicSoundClass" (`self.GetMusicValue`))
  (`GameplayStatics.SetSoundMixClassOverride` "/Game/Assets/Sounds/GameSoundClassMix.GameSoundClassMix" "/Game/Assets/Sounds/SFXSoundClass.SFXSoundClass" (`self.GetSFXValue`))
  (`GameplayStatics.PushSoundMixModifier` "/Game/Assets/Sounds/GameSoundClassMix.GameSoundClassMix"))

(fn `GameSave`
  (`self.SetupSaveInfo`)
  (bind _returnvalue (`GameplayStatics.LoadGameFromSlot` "RedemptionSave"))
  (bind _assave_data (cast `SaveData` _returnvalue)
    (:`then`
      (set `SaveData.SaveDataStruct` (`self.SaveInfo`) _assave_data)
      (`GameplayStatics.SaveGameToSlot` _assave_data "RedemptionSave"))
    (:`CastFailed`
      (bind _returnvalue_2 (`GameplayStatics.CreateSaveGameObject` "/Script/Redemption.SaveData"))
      (`GameplayStatics.SaveGameToSlot` _returnvalue_2 "RedemptionSave")))
  (`KismetSystemLibrary.PrintString` "Saved"))